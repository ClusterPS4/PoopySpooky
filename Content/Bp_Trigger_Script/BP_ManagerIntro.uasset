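; Intro manager actor scripting a one-time-style cutscene that hands over to gameplay, though its logic is unwired and BeginPlay is empty.
; The disconnected chain disables player input, blends to a focus camera, plays a level sequence, then restores view and input.
; It then spawns Bertha and Klemens through spawner references and activates a trigger.
; HasPlayed gates the chain but is set false at the end, so never latches.
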(event `self.ReceiveBeginPlay`)

(fn `UserConstructionScript`)