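; Trigger box that plays a one-shot cinematic when the first-person character overlaps it while active.
; It puts Bertha and the found MirrorGuys actor (Klemens) into cinematic visibility, disables input, blends to a cine camera and plays a level sequence.
; After the sequence's duration it teleports the player, blends back to the previous view, restores input and visibility, then triggers the Bertha and Klemens spawners.
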(event `self.Box.OnComponentBeginOverlap`
  (params (OverlappedComponent :type "PrimitiveComponent Object Reference") (OtherActor :type "Actor Object Reference") (OtherComp :type "PrimitiveComponent Object Reference") (OtherBodyIndex :type Integer) (bFromSweep :type Boolean) (SweepResult :type "HitResult Structure (by ref)"))
  ;[1 1 1] Olap start cinématique
  (if (`self.Is active`)
    (bind _asbp_first_person_character (cast `/Game/FirstPerson/Blueprints/BP_FirstPersonCharacter` OtherActor))
    (set `self.PlayerRef` _asbp_first_person_character)
    (bind _returnvalue (`GameplayStatics.GetActorOfClass` "/Game/Blueprints/AI/AIWalking/BP_MirrorGuys1.BP_MirrorGuys1_C"))
    (`/Engine/EditorBlueprintResources/StandardMacros.IsValid` _returnvalue
      (:`Is Valid`
        (set `self.Klemens` _returnvalue)
        (if (not (`self.HasPlayed`))
          (`/Game/Blueprints/AI/FlyingIATest/BP_FlyingPawnExample.EnterCine` (`self.Bertha`))
          (`/Game/Blueprints/AI/AIWalking/BP_MirrorGuys1.VisibleForCam` (`self.Klemens`))
          (`self.PlayCine`)
          (set `self.HasPlayed` true))))))

(event `PlayCine`
  (bind _returnvalue (`GameplayStatics.GetPlayerController` 0))
  (bind _sequenceplayer (`LevelSequenceActor.SequencePlayer` (`self.SequencerToPlay`)))
  ;[1 1 1] Play sequence : disable input -> Blend -> play seq -> for duration -> tp -> cam blend -> enable inputs
  (`self.DisableInput` (`self.PlayerRef`) _returnvalue)
  (set `self.CamToReturn` (`Controller.GetViewTarget` _returnvalue))
  (`PlayerController.SetViewTargetWithBlend` _returnvalue (`self.CamToBlend`) (`self.BlendTime`) "VTBlend_Linear" 0.0 false)
  (`MovieSceneSequencePlayer.Play` _sequenceplayer)
  (`KismetSystemLibrary.Delay` (`TimeManagementBlueprintLibrary.Conv_QualifiedFrameTimeToSeconds` (`MovieSceneSequencePlayer.GetDuration` _sequenceplayer)))
  (`self.K2_SetActorLocationAndRotation` (`self.PlayerRef`) (`self.LocTP2`) (`self.K2_GetActorRotation` (`self.CamToBlend`)) false false)
  (`PlayerController.SetViewTargetWithBlend` (`GameplayStatics.GetPlayerController` 0) (`self.CamToReturn`) (`self.BlendTime`) "VTBlend_Linear" 0.0 false)
  (`self.EnableInput` (`self.PlayerRef`) (`GameplayStatics.GetPlayerController` 0))
  (`/Game/Blueprints/AI/FlyingIATest/BP_FlyingPawnExample.ExitCine` (`self.Bertha`))
  (`/Game/Blueprints/AI/AIWalking/BP_MirrorGuys1.VisibilityForPlayer` (`self.Klemens`))
  ;[1 1 1] Spawn des monstres
  (`|ExecutionSequence`
    (:`then_0`
      (`/Game/Bp_Trigger_Script/Spawns/BP_SpawnBertha.Spawn Bertha` (`self.Spawn Bertha`)))
    (:`then_1`
      (`/Game/Bp_Trigger_Script/Spawns/BP_SpawnKlemens.Spawn` (`self.Spawn Klemens`)))))

(fn `UserConstructionScript`)