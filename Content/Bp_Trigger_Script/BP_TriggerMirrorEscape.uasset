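; A one-shot trigger actor that slides a piece of furniture when the first-person character enters its volume.
; The construction script applies per-instance mesh, start and target offsets, rotation, scale and trigger location.
; If Activate is set, player overlap clears it and plays a timeline.
; The timeline sets the furniture's relative location to the target position scaled by its track, not interpolated from the start offset.
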(event `self.Trigger.OnComponentBeginOverlap`
  (params (OverlappedComponent :type "PrimitiveComponent Object Reference") (OtherActor :type "Actor Object Reference") (OtherComp :type "PrimitiveComponent Object Reference") (OtherBodyIndex :type Integer) (bFromSweep :type Boolean) (SweepResult :type "HitResult Structure (by ref)"))
  (if (`self.Activate`)
    (cast `/Game/FirstPerson/Blueprints/BP_FirstPersonCharacter` OtherActor)
    (`/Engine/EditorBlueprintResources/StandardMacros.DoOnce` false
      (:`Completed`
        (set `self.Activate` false)
        (bind (_direction _newtrack_0) (`Timeline|Timeline`)
          (:`Update`
            (`SceneComponent.K2_SetRelativeLocation` (`self.Furniture`) (* _newtrack_0 (`SceneComponent.RelativeLocation` (`self.TargetPos`))) false false)))))))

(fn `UserConstructionScript`
  (bind _targetpos (`self.TargetPos`))
  (bind _furniture (`self.Furniture`))
  (bind _trigger (`self.Trigger`))
  (bind _furniture_2 (`self.Furniture`))
  (bind (_relativelocation_x _relativelocation_y _relativelocation_z) (`KismetMathLibrary.BreakVector` (`SceneComponent.RelativeLocation` _targetpos)))
  (bind (_relativerotation_roll _relativerotation_pitch _relativerotation_yaw) (`KismetMathLibrary.BreakRotator` (`SceneComponent.RelativeRotation` _furniture)))
  (bind (_relativelocation_x_2 _relativelocation_y_2 _relativelocation_z_2) (`KismetMathLibrary.BreakVector` (`SceneComponent.RelativeLocation` _furniture_2)))
  (`SceneComponent.K2_SetRelativeLocation` _targetpos (`KismetMathLibrary.MakeVector` (+ _relativelocation_x (`self.TargetX`)) (+ _relativelocation_y (`self.TargetY`)) (+ _relativelocation_z (`self.TargetYZ`))) false false)
  (`SceneComponent.K2_SetRelativeLocation` _furniture_2 (`KismetMathLibrary.MakeVector` (+ _relativelocation_x_2 (`self.StartX`)) (+ _relativelocation_y_2 (`self.StartY`)) (+ _relativelocation_z_2 (`self.StartZ`))) false false)
  (`SceneComponent.SetRelativeScale3D` _furniture_2 (* (`SceneComponent.RelativeScale3D` _furniture_2) (`self.ScaleMultiplier`)))
  (`StaticMeshComponent.SetStaticMesh` _furniture (`self.FurnitureToMove`))
  (`SceneComponent.K2_SetRelativeRotation` _furniture (`KismetMathLibrary.MakeRotator` (+ _relativerotation_roll (`self.RotationX`)) (+ _relativerotation_pitch (`self.RotationY`)) (+ _relativerotation_yaw (`self.RotationZ`))) false false)
  (`SceneComponent.K2_SetRelativeLocation` _trigger (+ (`SceneComponent.RelativeLocation` _trigger) (`self.TriggerLocation`)) false false))