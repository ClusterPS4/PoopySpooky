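; BP_SpawnKlemens spawns the mirror character Klemens (BP_MirrorGuys1) at its Box location.
; It caches any existing Klemens on BeginPlay; Spawn destroys that reference, creates a replacement and passes it Mirrors.
; AggroK enables aggro mode, with Final replacing Path if it is also the final trigger.
; A final trigger also makes Klemens visible in the real world and changes ambient sound through BP_SOUND.
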(event `self.ReceiveBeginPlay`
  (bind _returnvalue (`GameplayStatics.GetActorOfClass` "/Game/Blueprints/AI/AIWalking/BP_MirrorGuys1.BP_MirrorGuys1_C"))
  (set `self.Klemens` _returnvalue))

(event `Get actor for Klemens`
  (bind _returnvalue (`GameplayStatics.GetActorOfClass` "/Game/Blueprints/AI/AIWalking/BP_MirrorGuys1.BP_MirrorGuys1_C"))
  (set `self.Klemens` _returnvalue))

(event `Spawn`
  (bind _klemens (`self.Klemens`))
  (bind _klemens_2 (`self.Klemens`))
  (bind _klemens_3 (`self.Klemens`))
  (bind _klemens_4 (`self.Klemens`))
  ;[1 1 1] Spawn Klemens
  (`/Engine/EditorBlueprintResources/StandardMacros.IsValid` _klemens_2
    (:`Is Valid`
      (`self.K2_DestroyActor` _klemens_2))
    (:`Is Not Valid`
      _))
  (bind _returnvalue (`|SpawnActorFromClass` :`Class` "/Game/Blueprints/AI/AIWalking/BP_MirrorGuys1.BP_MirrorGuys1_C" :`SpawnTransform` (`KismetMathLibrary.MakeTransform` (`SceneComponent.K2_GetComponentLocation` (`self.Box`))) :`CollisionHandlingOverride` "Undefined" :`TransformScaleMethod` "OverrideRootScale" :`Instigator` null))
  (set `self.Klemens` _returnvalue)
  (set `/Game/Blueprints/AI/AIWalking/BP_MirrorGuys1.TouchMirror` (`self.Mirrors`) _klemens)
  (if (`self.AggroK`)
    (set `/Game/Blueprints/AI/AIWalking/BP_MirrorGuys1.AggroMode` true _klemens_3)
    (if (`self.isFinalTrigger`)
      (`/Game/Blueprints/AI/AIWalking/BP_MirrorGuys1.Final` _klemens_3)
      (else
        (`/Game/Blueprints/AI/AIWalking/BP_MirrorGuys1.Path` _klemens :!label _label)))
    (else
      (goto _label)))
  (if (`self.isFinalTrigger`)
    (set `/Game/Blueprints/AI/AIWalking/BP_MirrorGuys1.isVisibleRealWorld` true _klemens_4)
    (`/Game/Blueprints/AI/AIWalking/BP_MirrorGuys1.VisibilityForPlayer` _klemens_4)
    (bind _returnvalue_2 (`GameplayStatics.GetActorOfClass` "/Game/SFX/Cues/BP_SOUND.BP_SOUND_C"))
    (`/Game/SFX/Cues/BP_SOUND.ChangeAmbientSound` _returnvalue_2)))

(fn `UserConstructionScript`)