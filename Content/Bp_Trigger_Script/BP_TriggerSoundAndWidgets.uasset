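; Box trigger actor that shows subtitle text when the first-person character enters it while Activated, firing only once.
; It creates a Subtitle widget for either mid-screen text or bottom text with an optional follow-up line, removing each after a delay.
; Afterwards it can hand activation to another trigger, chaining them.
; A parallel Sequence branch optionally enables a mirror and its button without waiting for the subtitles.
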(event `self.Box.OnComponentBeginOverlap`
  (params (OverlappedComponent :type "PrimitiveComponent Object Reference") (OtherActor :type "Actor Object Reference") (OtherComp :type "PrimitiveComponent Object Reference") (OtherBodyIndex :type Integer) (bFromSweep :type Boolean) (SweepResult :type "HitResult Structure (by ref)"))
  (bind _subtitlewidget (`self.SubtitleWidget`))
  (bind _subtitlewidget_2 (`self.SubtitleWidget`))
  (bind _subtitlewidget_3 (`self.SubtitleWidget`))
  ;[1 1 1] Detection player dans box Collider
  (if (`self.Activated`)
    (cast `/Game/FirstPerson/Blueprints/BP_FirstPersonCharacter` OtherActor)
    (`/Engine/EditorBlueprintResources/StandardMacros.DoOnce` false
      (:`Completed`
        ;[1 1 1] Attribution du Widget
        (bind _returnvalue (`|CreateWidget` "/Game/LevelPrototyping/WidgetSubtitle/Subtitle.Subtitle_C" (`GameplayStatics.GetPlayerController` 0)))
        (set `self.subtitlewidget` _returnvalue)
        ;[1 1 1] Si le texte est au milieu de l'écran on l'affiche, sinon on passe au texte en bas de l'écran
        (`|ExecutionSequence`
          (:`then_0`
            (if (`self.TextIsMidScreen`)
              (set `/Game/LevelPrototyping/WidgetSubtitle/Subtitle.Setcommand` (`self.WidgText`) _subtitlewidget_2)
              (`UserWidget.AddToViewport` _subtitlewidget_2 0)
              (`KismetSystemLibrary.Delay` 3.0)
              (`Widget.RemoveFromParent` _subtitlewidget_2)
              ;[1 1 1] Activation du trigger suivant
              (if (`self.ActivateOtherTrigger`)
                (set `/Game/Bp_Trigger_Script/BP_TriggerSoundAndWidgets.Activated` true (`self.TrggerToActivate`))
                (set `self.Activated` false))
              (else
                ;[1 1 1] Attibution du texte et affichage pendant 3 secondes
                (set `/Game/LevelPrototyping/WidgetSubtitle/Subtitle.TextToSet` (`self.WidgText`) _subtitlewidget)
                (`UserWidget.AddToViewport` _subtitlewidget 0)
                (`KismetSystemLibrary.Delay` 3.0)
                (`Widget.RemoveFromParent` _subtitlewidget)
                ;[1 1 1] Affichage du second texte si besoin
                (if (`self.FollowUpText`)
                  (set `/Game/LevelPrototyping/WidgetSubtitle/Subtitle.TextToSet` (`self.WidgText2`) _subtitlewidget_3)
                  (`UserWidget.AddToViewport` _subtitlewidget_3 0)
                  (`KismetSystemLibrary.Delay` 3.0)
                  (`Widget.RemoveFromParent` _subtitlewidget_3)
                  ;[1 1 1] Activation du trigger suivant
                  (if (`self.ActivateOtherTrigger`)
                    (set `/Game/Bp_Trigger_Script/BP_TriggerSoundAndWidgets.Activated` true (`self.TrggerToActivate`))
                    (set `self.Activated` false))
                  (else
                    ;[1 1 1] Activation du trigger suivant
                    (if (`self.ActivateOtherTrigger`)
                      (set `/Game/Bp_Trigger_Script/BP_TriggerSoundAndWidgets.Activated` true (`self.TrggerToActivate`))
                      (set `self.Activated` false)))))))
          (:`then_1`
            (if (`self.Activate miror`)
              (set `/Game/Blueprints/Miroirs/BP_Mirror.Activable` true (`self.Miror to activate`))
              (set `/Game/Bp_Trigger_Script/BP_PrintBoutonE.Ready` true (`self.boutonEtoActivate`)))))))))

(fn `UserConstructionScript`)