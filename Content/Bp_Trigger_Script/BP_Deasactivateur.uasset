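; BP_Deasactivateur is a trigger volume that repositions and respawns the player's flying pawn when that pawn enters its box.
; On BeginPlay it caches the level's BP_FlyingPawnExample as BigBertha.
; On overlap by that pawn class, it moves BigBertha to the box location of the TempSpawn reference, assigns SplineToFollow as its spline and calls its Spawn function.
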(event `self.ReceiveBeginPlay`
  (bind _returnvalue (`GameplayStatics.GetActorOfClass` "/Game/Blueprints/AI/FlyingIATest/BP_FlyingPawnExample.BP_FlyingPawnExample_C"))
  (set `self.BigBertha` _returnvalue))

(event `self.Box.OnComponentBeginOverlap`
  (params (OverlappedComponent :type "PrimitiveComponent Object Reference") (OtherActor :type "Actor Object Reference") (OtherComp :type "PrimitiveComponent Object Reference") (OtherBodyIndex :type Integer) (bFromSweep :type Boolean) (SweepResult :type "HitResult Structure (by ref)"))
  (bind _bigbertha (`self.BigBertha`))
  (cast `/Game/Blueprints/AI/FlyingIATest/BP_FlyingPawnExample` OtherActor)
  (`self.K2_SetActorLocation` (`self.BigBertha`) (`SceneComponent.K2_GetComponentLocation` (`/Game/Blueprints/AI/FlyingIATest/Temp_Spawn.Box` (`self.TempSpawn`))) false false)
  (set `/Game/Blueprints/AI/FlyingIATest/BP_FlyingPawnExample.FollowSpline` (`self.SplineToFollow`) _bigbertha)
  (`/Game/Blueprints/AI/FlyingIATest/BP_FlyingPawnExample.Spawn` _bigbertha null))

(fn `UserConstructionScript`)