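; An end-of-game trigger box that rolls the credits when the first-person character overlaps it, then opens the UI_Menu level.
; While active, it runs once, stopping the sound, moving the player to a fixed location, disabling input and adding the credits widget.
; A timeline paced by TimeToTravel scrolls the widget's credit image vertically, clears IsActive as it updates, and loads the menu when finished.
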(event `self.Box.OnComponentBeginOverlap`
  (params (OverlappedComponent :type "PrimitiveComponent Object Reference") (OtherActor :type "Actor Object Reference") (OtherComp :type "PrimitiveComponent Object Reference") (OtherBodyIndex :type Integer) (bFromSweep :type Boolean) (SweepResult :type "HitResult Structure (by ref)"))
  (bind _playerref (`self.playerref`))
  (if (`self.isActive`)
    (bind _asbp_first_person_character (cast `/Game/FirstPerson/Blueprints/BP_FirstPersonCharacter` OtherActor))
    (set `self.playerref` _asbp_first_person_character)
    (`/Engine/EditorBlueprintResources/StandardMacros.DoOnce` false
      (:`Completed`
        (`/Game/SFX/Cues/BP_SOUND.StopSound` (`self.Sound`))
        (`self.K2_SetActorLocation` _playerref (-3065.0 5211.0 -789.0) false false)
        (`self.DisableInput` _playerref (`GameplayStatics.GetPlayerController` 0))
        (bind _returnvalue (`|CreateWidget` "/Game/UI/WG_Credtis.WG_Credtis_C"))
        (`UserWidget.AddToViewport` _returnvalue 0)
        (`TimelineComponent.SetPlayRate` (`self.Credit`) (/ 1.0 (`self.Time to travel`)))
        (bind (_direction _newtrack_0) (`Timeline|Credit` :!via `PlayFromStart`)
          (:`Update`
            (`Widget.SetRenderTranslation` (`/Game/UI/WG_Credtis.Image_Credit` _returnvalue) (`KismetMathLibrary.MakeVector2D` 0.0 (* _newtrack_0 1080.0)))
            (set `self.isActive` false))
          (:`Finished`
            (`GameplayStatics.OpenLevelBySoftObjectPtr` "/Game/LDTest/UI_Menu.UI_Menu")))))))

(fn `UserConstructionScript`)