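; Trigger actor that teleports the first-person player to the final corridor for the end sequence.
; When active and overlapped by the player, it fires once, deactivating itself and moving the player to its PlayerSpawn component's location.
; It also unequips the mirror, disables stamina and sets Cinemens visible in the real world.
; The construction script shifts PlayerSpawn by the PSpawn X, Y and Z offset variables.
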(event `self.ReceiveBeginPlay`
  ;[1 1 1] Set player Ref
  (bind _returnvalue (`GameplayStatics.GetActorOfClass` "/Game/FirstPerson/Blueprints/BP_FirstPersonCharacter.BP_FirstPersonCharacter_C"))
  (set `self.Player` _returnvalue))

(event `self.Trigger.OnComponentBeginOverlap`
  (params (OverlappedComponent :type "PrimitiveComponent Object Reference") (OtherActor :type "Actor Object Reference") (OtherComp :type "PrimitiveComponent Object Reference") (OtherBodyIndex :type Integer) (bFromSweep :type Boolean) (SweepResult :type "HitResult Structure (by ref)"))
  (bind _player (`self.Player`))
  ;[1 1 1] TP player dans couloir final
  (if (`self.Activcable`)
    (cast `/Game/FirstPerson/Blueprints/BP_FirstPersonCharacter` OtherActor)
    (`/Engine/EditorBlueprintResources/StandardMacros.DoOnce` false
      (:`Completed`
        (set `self.Activcable` false)
        (`self.K2_SetActorLocation` _player (`SceneComponent.K2_GetComponentLocation` (`self.PlayerSpawn`)) false false)
        (`/Game/FirstPerson/Blueprints/BP_FirstPersonCharacter.UnequipMiror` _player)
        (set `/Game/Blueprints/AI/AIWalking/BP_KlemensCinmatique.isVisibleRealWorld` true (`self.Cinemens`))
        (set `/Game/FirstPerson/Blueprints/BP_FirstPersonCharacter.IsStaminaActive` false (`self.Player`))))))

(fn `UserConstructionScript`
  (bind _playerspawn (`self.PlayerSpawn`))
  (bind (_relativelocation_x _relativelocation_y _relativelocation_z) (`KismetMathLibrary.BreakVector` (`SceneComponent.RelativeLocation` _playerspawn)))
  (`SceneComponent.K2_SetRelativeLocation` _playerspawn (`KismetMathLibrary.MakeVector` (+ _relativelocation_x (`self.PSpawnX`)) (+ _relativelocation_y (`self.PSpawnY`)) (+ _relativelocation_z (`self.PSpawnZ`))) false false))