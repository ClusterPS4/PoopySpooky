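; BP_Corde is a chain, filed under the salon puzzle, built from instanced link meshes along a spline.
; CreateChain runs at construction, spacing links by mesh bounds plus an offset and alternating yaw and position offsets to interlock them.
; Lift extends the spline's second point downward, rebuilds the chain and lowers the actor's root through a timeline.
; Reduce drives the root's relative height from the Up timeline without rebuilding links.
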(event `self.ReceiveBeginPlay`)

(event `Lift`
  (bind _spline (`self.Spline`))
  (bind (_returnvalue_x _returnvalue_y _returnvalue_z) (`KismetMathLibrary.BreakVector` (`SplineComponent.GetLocationAtSplinePoint` _spline 1 "Local")))
  (`InstancedStaticMeshComponent.ClearInstances` (`self.InstancedStaticMesh`))
  (`SplineComponent.SetLocationAtSplinePoint` _spline 1 (`KismetMathLibrary.MakeVector` _returnvalue_x _returnvalue_y (+ _returnvalue_z (* (`self.EspaceMaillons`) -13.0))) "Local" true)
  (`self.CreateChain`)
  (`Timeline|Timeline`
    (:`Update`
      (`SceneComponent.K2_AddWorldOffset` (`self.DefaultSceneRoot`) (0.0 0.0 -0.1) false false))))

(event `Reduce`
  (bind _defaultsceneroot (`self.DefaultSceneRoot`))
  (bind (_relativelocation_x _relativelocation_y) (`KismetMathLibrary.BreakVector` (`SceneComponent.RelativeLocation` _defaultsceneroot)))
  (bind (_direction _newtrack_0) (`Timeline|Up`)
    (:`Update`
      (`SceneComponent.K2_SetRelativeLocation` _defaultsceneroot (`KismetMathLibrary.MakeVector` _relativelocation_x _relativelocation_y _newtrack_0) false false))))

(fn `CreateChain`
  (bind (_min _max) (break `Box` (`StaticMesh.GetBoundingBox` (`self.Maillon`))))
  ;[1 0.3231 0.2462] (J'avoue j'ai regardé un tuto pour ça)
  ;;[1 1 1] Attribution d'un static mesh à l'instance
  (`StaticMeshComponent.SetStaticMesh` (`self.InstancedStaticMesh`) (`self.Maillon`))
  (bind _output_get (set `self.EspaceMaillons` (+ (.y (- _max _min)) (`self.Offset`))))
  ;;[1 1 1] On pose les maillons 1 par 1
  (bind _output_get_2 (set `self.Nombre de maillons` (`KismetMathLibrary.FFloor` (/ (`SplineComponent.GetSplineLength` (`self.Spline`)) _output_get))))
  (for _index (range (+ _output_get_2 1))
    ;;[1 0.3231 0.2462] (Sauf pour ça, j'ai improvisé)
    ;;;[1 1 1] On modifie la rotation d'un maillon sur deux
    (if (== (mod _index 2) 0)
      (set `self.RotationMaillons` 0.0)
      ;;;[1 1 1] On modifie leur offset sur la spline car le pivot n'est pas au milieu
      (set `self.LocationMaillonsX` -6.5)
      (set `self.LocationMaillonsY` 0.0)
      (else
        (set `self.RotationMaillons` 90.0)
        (set `self.LocationMaillonsX` 0.0)
        (set `self.LocationMaillonsY` 6.5)))
    (bind (_returnvalue_x _returnvalue_y _returnvalue_z) (`KismetMathLibrary.BreakVector` (`SplineComponent.GetLocationAtDistanceAlongSpline` (`self.Spline`) (* _index (`self.EspaceMaillons`)) "Local")))
    ;;[1 1 1] On ajoute l'instance au static mesh à la bonne position
    (`InstancedStaticMeshComponent.AddInstance` (`self.InstancedStaticMesh`) (`KismetMathLibrary.MakeTransform` (`KismetMathLibrary.MakeVector` (+ _returnvalue_x (`self.LocationMaillonsX`)) (+ _returnvalue_y (`self.LocationMaillonsY`)) _returnvalue_z) (`KismetMathLibrary.MakeRotator` 90.0 0.0 (`self.RotationMaillons`))) false)))

(fn `UserConstructionScript`
  (`self.CreateChain`))