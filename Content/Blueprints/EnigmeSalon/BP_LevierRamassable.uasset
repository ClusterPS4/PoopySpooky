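; BP_LevierRamassable is a lever pickup for the salon puzzle (EnigmeSalon) that can be collected only after it is revealed.
; The construction script hides the Levier component and clears IsVisible; the Reveal event makes Box visible and sets the flag.
; When IsVisible is true, the Interactable event sets HasLever on the player's BP_FirstPersonCharacter and destroys the actor.
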(event `/Game/Blueprints/BPI_Reveal.Reveal`
  (`SceneComponent.SetVisibility` (`self.Box`) true false)
  (set `self.IsVisible` true))

(event `/Game/Blueprints/BPI_Interactable.Interactable`
  (params (Actor :type "Actor Object Reference"))
  (if (`self.IsVisible`)
    (bind _asbp_first_person_character (cast `/Game/FirstPerson/Blueprints/BP_FirstPersonCharacter` (`GameplayStatics.GetPlayerCharacter` 0)))
    (set `/Game/FirstPerson/Blueprints/BP_FirstPersonCharacter.HasLever` true _asbp_first_person_character)
    (`self.K2_DestroyActor`)))

(fn `UserConstructionScript`
  (`SceneComponent.SetVisibility` (`self. Levier`) false false)
  (set `self.IsVisible` false))