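; Lever-operated lift machine for the salon puzzle that raises a chandelier and makes a key gatherable.
; Interacting first reveals the hidden lever if it has been gathered, then a further interaction runs the one-shot Lift.
; A lever-pull timeline leads into simultaneous gear-rotation and lift timelines, the latter scaling the rope and moving the chandelier.
; The key snaps to its new height as those start, using hardcoded X/Y positions like the chandelier.
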(event `/Game/Blueprints/BPI_Interactable.Interactable`
  (params (Actor :type "Actor Object Reference"))
  ;[1 1 1] Interract -> Placement du levier / lift
  (if (`self.LeverIn`)
    (`self.Lift`)
    (elif (`self.LeverGathered`)
      (`SceneComponent.SetVisibility` (`self.Levier`) true false)
      (set `self.LeverIn` true))))

(event `Lift`
  ;[1 1 1] Verif si le levier est activé
  (if (`self.IsDown`)
    (set `self.IsDown` false)
    ;[1 1 1] Activation levier
    (bind (_direction _newtrack_0) (`Timeline|LeverPull`)
      (:`Update`
        (`SceneComponent.K2_SetRelativeRotation` (`self.Levier`) (`KismetMathLibrary.MakeRotator` 0.0 _newtrack_0) false false))
      (:`Finished`
        (`|ExecutionSequence`
          (:`then_0`
            ;[1 1 1] Ratation Gears
            (bind (_direction_2 _newtrack_0_2) (`Timeline|RotatiionGears`)
              (:`Update`
                (bind _returnvalue (* _newtrack_0_2 (`self.RatationGears360`)))
                (`SceneComponent.K2_SetRelativeRotation` (`self.GearC`) (`KismetMathLibrary.MakeRotator` 0.0 _returnvalue) false false)
                (`SceneComponent.K2_SetRelativeRotation` (`self.GearA`) (`KismetMathLibrary.MakeRotator` 0.0 (* _returnvalue -1.0)) false false)
                (`SceneComponent.K2_SetRelativeRotation` (`self.GearB`) (`KismetMathLibrary.MakeRotator` 0.0 (* (* _newtrack_0_2 (`self.RotationGear180`)) -1.0)) false false))))
          (:`then_1`
            ;[1 1 1] Lift Chandelier
            (bind (_direction_3 _newtrack_0_3) (`Timeline|LiftUp`)
              (:`Update`
                (`self.SetActorRelativeScale3D` (`self.RopeToInterract`) (`KismetMathLibrary.MakeVector` 1.0 1.0 (* _newtrack_0_3 (`self.ScaleFactor`))))
                (`SceneComponent.K2_SetRelativeLocation` (`/Game/Blueprints/EnigmeSalon/BP_Chandelier.DefaultSceneRoot` (`self.Chandelier`)) (`KismetMathLibrary.MakeVector` -2958.0 -319.0 (* _newtrack_0_3 (`self.NewHeight`))) false false))))
          (:`then_2`
            ;[1 1 1] Descendre Clef
            (`SceneComponent.K2_SetRelativeLocation` (`/Game/Blueprints/EnigmeSalon/BP_KeyActivator.DefaultSceneRoot` (`self.KeyToDown`)) (`KismetMathLibrary.MakeVector` -2723.0 -1373.0 (`self.KeyHeight`)) false false)
            (set `/Game/Blueprints/EnigmeSalon/BP_KeyActivator.Is gatherable` true (`self.KeyToDown`))))))))

(fn `UserConstructionScript`
  (`SceneComponent.SetVisibility` (`self.Levier`) false false))