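; BP_Key is a key pickup that the first-person player collects through its Interactable event.
; Three boolean flags, checked in order, select which key enum value the actor represents.
; The selected value is added uniquely to the KeyEnum array on BP_FirstPersonCharacter, then the key destroys itself.
; If no flag is set or the character cast fails, the key stays in place.
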(event `/Game/Blueprints/BPI_Interactable.Interactable`
  (if (`self.IsKey1`)
    (bind _asbp_first_person_character (cast `/Game/FirstPerson/Blueprints/BP_FirstPersonCharacter` (`GameplayStatics.GetPlayerCharacter` 0)))
    (`KismetArrayLibrary.Array_AddUnique` (`/Game/FirstPerson/Blueprints/BP_FirstPersonCharacter.KeyEnum` _asbp_first_person_character) "NewEnumerator0")
    (`self.K2_DestroyActor`)
    (elif (`self.IsKey2`)
      (bind _asbp_first_person_character_2 (cast `/Game/FirstPerson/Blueprints/BP_FirstPersonCharacter` (`GameplayStatics.GetPlayerCharacter` 0)))
      (`KismetArrayLibrary.Array_AddUnique` (`/Game/FirstPerson/Blueprints/BP_FirstPersonCharacter.KeyEnum` _asbp_first_person_character_2) "NewEnumerator1")
      (`self.K2_DestroyActor`)
      (elif (`self.IsKey3`)
        (bind _asbp_first_person_character_3 (cast `/Game/FirstPerson/Blueprints/BP_FirstPersonCharacter` (`GameplayStatics.GetPlayerCharacter` 0)))
        (`KismetArrayLibrary.Array_AddUnique` (`/Game/FirstPerson/Blueprints/BP_FirstPersonCharacter.KeyEnum` _asbp_first_person_character_3) "NewEnumerator2")
        (`self.K2_DestroyActor`)))))

(fn `UserConstructionScript`)