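; BP_DoubleDoor is a double door that toggles open and closed through its Interactable event, which does nothing while IsLocked is set.
; Interactable flips Isopen and plays or reverses the OpenAngle timeline.
; Each timeline update lerps yaw from zero to Angle on StaticMesh and applies the negated yaw to SMDoorMirror, so the two leaves swing as mirror images.
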(event `/Game/Blueprints/BPI_Interactable.Interactable`
  (if (`self.IsLocked`)
    _
    (elif (`self.Isopen`)
      (set `self.Isopen` false)
      (bind (_direction _newtrack_0) (`Timeline|OpenAngle` :!via `Reverse` :!label _label)
        (:`Update`
          (bind _returnvalue (`KismetMathLibrary.Lerp` 0.0 (`self.Angle`) _newtrack_0))
          (`SceneComponent.K2_SetRelativeRotation` (`self.StaticMesh`) (`KismetMathLibrary.MakeRotator` 0.0 0.0 _returnvalue) false false)
          (`SceneComponent.K2_SetRelativeRotation` (`self.SM_DoorMirror`) (`KismetMathLibrary.MakeRotator` 0.0 0.0 (* _returnvalue -1.0)) false false)))
      (else
        (set `self.Isopen` true)
        (goto _label)))))

(fn `UserConstructionScript`)