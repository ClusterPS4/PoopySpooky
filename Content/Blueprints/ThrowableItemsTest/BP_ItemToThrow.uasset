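; BP_ItemToThrow is a test throwable item that makes noise when it hits something.
; On a static mesh hit, it checks that the mesh's upward Z velocity exceeds a threshold, so downward motion does not pass.
; It then calls MakeNoise at the mesh location with the first-person player character as instigator, using loudness and range variables, and prints a debug string.
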(event `self.StaticMesh.OnComponentHit`
  (params (HitComponent :type "PrimitiveComponent Object Reference") (OtherActor :type "Actor Object Reference") (OtherComp :type "PrimitiveComponent Object Reference") (NormalImpulse :type "Vector Structure") (Hit :type "HitResult Structure (by ref)"))
  ;[1 1 1] HitEventWithSpeed
  (bind _staticmesh (`self.StaticMesh`)
    (:`then`
      (bind (_returnvalue_x _returnvalue_y _returnvalue_z) (`KismetMathLibrary.BreakVector` (`SceneComponent.GetComponentVelocity` _staticmesh)))
      (if (> _returnvalue_z 100.0)
        (bind _asbp_first_person_character (cast `/Game/FirstPerson/Blueprints/BP_FirstPersonCharacter` (`GameplayStatics.GetPlayerPawn` 0)))
        (bind _output_get (set `self.PlayerRef` _asbp_first_person_character))
        (`self.MakeNoise` self (`self.Loudness`) _output_get (`SceneComponent.K2_GetComponentLocation` (`self.StaticMesh`)) (`self.Max Range`) "None")
        (`KismetSystemLibrary.PrintString` "Hello")))
    (:`else`)))

(fn `UserConstructionScript`)