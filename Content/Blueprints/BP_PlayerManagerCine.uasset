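; BP_PlayerManagerCine is a helper that exposes player camera bop and character movement toggles, apparently for cinematics.
; It caches the BP_FirstPersonCharacter on BeginPlay, and EnableBop and DisableBop start or cancel that character's shake.
; KlemensIdle and KlemensMove write a zero or fixed non-zero velocity straight into the Cinemens character's movement component rather than feeding movement input.
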(event `self.ReceiveBeginPlay`
  (bind _returnvalue (`GameplayStatics.GetActorOfClass` "/Game/FirstPerson/Blueprints/BP_FirstPersonCharacter.BP_FirstPersonCharacter_C"))
  (set `self.PlayerRef` _returnvalue))

(event `EnableBop`
  (`/Game/FirstPerson/Blueprints/BP_FirstPersonCharacter.Start Shake` (`self.PlayerRef`)))

(event `DisableBop`
  (`/Game/FirstPerson/Blueprints/BP_FirstPersonCharacter.Cancel Shake` (`self.PlayerRef`)))

(event `KlemensIdle`
  (set `MovementComponent.Velocity` (0.0 0.0 0.0) (`Character.CharacterMovement` (`self.Cinemens`))))

(event `KlemensMove`
  (set `MovementComponent.Velocity` (50.0 50.0 50.0) (`Character.CharacterMovement` (`self.Cinemens`))))

(fn `UserConstructionScript`)