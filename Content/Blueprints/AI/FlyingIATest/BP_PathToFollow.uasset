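; Spline path actor for the flying AI test, providing a moving reference point for BP_FlyingPawnExample.
; While unlocked and the pawn is on the spline, Tick advances ReferencePoint by speed, optionally looping; Resetdistance returns it to the start.
; GetNearestPointOnSpline scans spline points for the one closest to the pawn's capsule and returns its world position.
; An alternative timeline-driven MoveAI is unconnected and marked as not working.
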(event `Move AI`
  (params (`AI Ref` :type "/Game/Blueprints/AI/FlyingIATest/BP_FlyingPawnExample Object Reference"))
  ;[1 1 1] Test New Spline ( Marche pas)
)

(event `self.ReceiveBeginPlay`
  (bind _returnvalue (`GameplayStatics.GetActorOfClass` "/Game/Blueprints/AI/FlyingIATest/BP_FlyingPawnExample.BP_FlyingPawnExample_C"))
  (set `self.Flying Ai Ref` _returnvalue))

(event `self.ReceiveTick`
  (params (DeltaSeconds :type "Float (single-precision)"))
  (bind (_returnvalue_location _returnvalue_rotation) (`KismetMathLibrary.BreakTransform` (`SplineComponent.GetTransformAtDistanceAlongSpline` (`self.TheSpline`) (`self.Distance`) "Local" false)))
  ;[0.4538 1 0.6823] Old Spline
  (if (`self.Locked`)
    _
    (elif (`/Game/Blueprints/AI/FlyingIATest/BP_FlyingPawnExample.IsOnSpline?` (`self.Flying Ai Ref`))
      (set `self.Distance` (+ (* DeltaSeconds (`self.Speed`)) (`self.Distance`)))
      (`SceneComponent.K2_SetRelativeTransform` (`self.referencePoint`) (`KismetMathLibrary.MakeTransform` _returnvalue_location _returnvalue_rotation (`SceneComponent.RelativeScale3D` (`self.referencePoint`))) false false)
      (if (`self.IsLooping`)
        (if (> (`self.Distance`) (`SplineComponent.GetSplineLength` (`self.TheSpline`)))
          (set `self.Distance` 0.0))))))

(event `Reset distance`
  (bind (_returnvalue_location _returnvalue_rotation) (`KismetMathLibrary.BreakTransform` (`SplineComponent.GetTransformAtDistanceAlongSpline` (`self.TheSpline`) (`self.Distance`) "Local" false)))
  ;[0.1667 1 0.2621] Reset Spline to Start
  (set `self.Distance` 0.0)
  (`SceneComponent.K2_SetRelativeTransform` (`self.referencePoint`) (`KismetMathLibrary.MakeTransform` _returnvalue_location _returnvalue_rotation (`SceneComponent.RelativeScale3D` (`self.referencePoint`))) false false))

(event `GetNearestPointOnSpline`
  (for _index (range (+ (`SplineComponent.GetNumberOfSplinePoints` (`self.TheSpline`)) 1))
    (bind _returnvalue (`KismetMathLibrary.Vector_Distance` (`SplineComponent.GetLocationAtSplinePoint` (`self.TheSpline`) _index "World") (`SceneComponent.K2_GetComponentLocation` (`Character.CapsuleComponent` (`self.Flying Ai Ref`)))))
    (if (> (`self.ShortestDistance`) _returnvalue)
      (set `self.ShortestDistance` _returnvalue))))

(fn `Get Nearest Point on Spline`
  (returns (NewParam :type Boolean) (ClosePointPosition :type "Vector Structure"))
  (bind _thespline (`self.TheSpline`))
  (for _index (range (+ (`SplineComponent.GetNumberOfSplinePoints` _thespline) 1))
    (bind _returnvalue (`KismetMathLibrary.Vector_Distance` (`SplineComponent.GetLocationAtSplinePoint` (`self.TheSpline`) _index "World") (`SceneComponent.K2_GetComponentLocation` (`Character.CapsuleComponent` (`self.Flying Ai Ref`)))))
    (if (> (`self.ShortestDistance`) _returnvalue)
      (set `self.ShortestDistance` _returnvalue)
      (set `self.KeepClosePointIndex` _index)))
  (return false (`SplineComponent.GetLocationAtSplinePoint` _thespline (`self.KeepClosePointIndex`) "World")))

(fn `UserConstructionScript`)