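; Actor that holds candidate destination points for the mirror AI and picks those nearest the player.
; Construction script previews each point with a box component and a persistent debug line from the actor.
; GetCloserPoint sorts the points by player distance with an early-exit bubble sort.
; It then fills PointNextToPlayer, up to a maximum count, with points passing a height check against the player's capsule bottom and WallHeight.
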(event `self.ReceiveBeginPlay`
  (bind _returnvalue (`GameplayStatics.GetActorOfClass` "/Game/FirstPerson/Blueprints/BP_FirstPersonCharacter.BP_FirstPersonCharacter_C"))
  (set `self.PlayerRef` _returnvalue)
  (bind _returnvalue_2 (`GameplayStatics.GetActorOfClass` "/Game/Blueprints/AI/AIWalking/BP_MirrorGuys1.BP_MirrorGuys1_C"))
  (set `self.AiMirror` _returnvalue_2))

(event `GetCloserPoint`
  (bind _allpointdestinationsmirror (`self.AllPointDestinationsMirror`))
  (bind (_origin _boxextent) (`KismetSystemLibrary.GetComponentBounds` (`Character.CapsuleComponent` (`self.PlayerRef`))))
  (bind (_returnvalue_x _returnvalue_y _returnvalue_z) (`KismetMathLibrary.BreakVector` (- (.z _origin) (.z _boxextent))))
  (`KismetArrayLibrary.Array_Clear` (`self.PointNextToPlayer`))
  (`self.SortVectorsByDistanceBubble` _allpointdestinationsmirror)
  (for _array_element _allpointdestinationsmirror
    (bind (_x _y _z) (`KismetMathLibrary.BreakVector3f` _array_element))
    (if (and (> _z _returnvalue_z) (< (+ _returnvalue_z (`self.WallHeight`)) _z) (< (`KismetArrayLibrary.Array_Length` (`self.PointNextToPlayer`)) (`self.Number Of Max Destination`)))
      (`KismetArrayLibrary.Array_Add` (`self.PointNextToPlayer`) _array_element))))

(fn `SortVectorsByDistanceBubble`
  (params (VectorsToSort :type "Array of Vector Structure (by ref)"))
  (locals (LastIndex :type Integer) (PlayerLocation :type "Vector Structure") (Swapped :type Boolean) (J :type Integer))
  (bind _j (`local.J`))
  ;[1 1 1] Init des variables (pas besoin d'avoir un tableau temp, on travaille direct sur vectorsToSort)
  (set `local.LastIndex` (`KismetArrayLibrary.Array_LastIndex` VectorsToSort))
  (set `local.PlayerLocation` (`self.K2_GetActorLocation` (`GameplayStatics.GetPlayerCharacter` 0)))
  (for _index (range (`local.LastIndex`))
    (set `local.Swapped` false)
    (for _index_2 (range (+ (- (`local.LastIndex`) _index 1) 1))
      (set `local.J` _index_2)
      (if (> (`KismetMathLibrary.Vector_Distance` (`|GetArrayItem` (`local.VectorsToSort`) (`local.J`)) (`local.PlayerLocation`)) (`KismetMathLibrary.Vector_Distance` (`|GetArrayItem` (`local.VectorsToSort`) (+ (`local.J`) 1)) (`local.PlayerLocation`)))
        ;[1 1 1] On swap
        (`KismetArrayLibrary.Array_Swap` (`local.VectorsToSort`) _j (+ _j 1))
        (set `local.Swapped` true)))
    ;[1 1 1] Opti, si pas eu de swap, on arrete
    (if (not (`local.Swapped`))
      (return)))
  (return))

(fn `UserConstructionScript`
  (`KismetSystemLibrary.FlushPersistentDebugLines`)
  (for _array_element (`self.AllPointDestinationsMirror`)
    (`AddComponent|NODE_AddBoxComponent-1` :`RelativeTransform` (`KismetMathLibrary.MakeTransform` _array_element))
    (`KismetSystemLibrary.DrawDebugLine` (`self.K2_GetActorLocation`) (`KismetMathLibrary.TransformLocation` (`self.GetTransform`) _array_element) (struct :`G` 0.1521 :`B` 1.0 :`A` 1.0) 99.0 10.0)))