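; AI character that roams between mirror destination points, favouring those near the player.
; It bubble-sorts BP_DestinationAiMirror's points by player distance, keeps up to three below a player-relative height limit, excluding the last watched spot, and picks one randomly.
; After each move it randomly either moves on or runs a debug-drawn sphere trace and pauses first, unless PlayerDetected halts the loop.
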(event `ContinuMoving`
  (bind _pointnearbyplayer (`self.PointNearbyPlayer`))
  (bind _returnvalue (`SceneComponent.K2_GetComponentLocation` (`self.Cone`)))
  (`self.DetectClosePointsPlayer` :!label _label)
  (if (!= (`KismetArrayLibrary.Array_Length` _pointnearbyplayer) 0)
    (bind _output_get (set `self.GoalDestination` (`KismetArrayLibrary.Array_Random` _pointnearbyplayer)))
    (else
      (set `self.GoalDestination` (`KismetArrayLibrary.Array_Random` (`self.All Point Destinations`)))))
  (`AITask_MoveTo.AIMoveTo` (cast `AIController` (`self.GetController`) :!pure true) (`KismetMathLibrary.TransformLocation` (`self.GetTransform` (stale `self.ReceiveBeginPlay` _returnvalue)) _output_get) null 50.0 "Enable" "Enable" true false false "Enable"
    (:`OnRequestFailed`
      (`self.ContinuMoving`))
    (:`OnMoveFinished`
      (if (not (`self.Player Detected`))
        (bind _output_get_2 (set `self.WatchMirror` (`KismetMathLibrary.RandomBool`)))
        (if _output_get_2
          (`KismetSystemLibrary.SphereTraceSingle` :`Start` _returnvalue :`End` (+ _returnvalue (* (`SceneComponent.GetForwardVector` (`self.Sphere`)) (`self.RayCastDist`))) :`Radius` 25.0 :`TraceChannel` "TraceTypeQuery1" :`DrawDebugType` "ForDuration")
          (set `self.TempActualLocation` (`self.GoalDestination`))
          (`KismetSystemLibrary.Delay` 2.0)
          (`self.ContinuMoving`)
          (else
            (`self.ContinuMoving`)))))))

(event `self.ReceiveBeginPlay`
  (bind _asbp_first_person_character (cast `/Game/FirstPerson/Blueprints/BP_FirstPersonCharacter` (`GameplayStatics.GetPlayerCharacter` 0)))
  (set `self.PlayerRef` _asbp_first_person_character)
  (bind _returnvalue (`GameplayStatics.GetActorOfClass` "/Game/Blueprints/AI/AIWalking/BP_DestinationAiMirror.BP_DestinationAiMirror_C"))
  (set `self.All Point Destinations` (`/Game/Blueprints/AI/AIWalking/BP_DestinationAiMirror.AllPointDestinationsMirror` _returnvalue))
  (goto _label))

(event `DetectClosePointsPlayer`
  (bind _actuallynearbypoint (`self.ActuallyNearbyPoint`))
  (bind _playerref (`self.PlayerRef`))
  (bind (_returnvalue_x _returnvalue_y _returnvalue_z) (`KismetMathLibrary.BreakVector` (`self.K2_GetActorLocation` _playerref)))
  ;[1 1 1] Récupère les 2 point le plus proche du player
  (`self.SortVectorsByDistance` (`self.All Point Destinations`))
  (`KismetArrayLibrary.Array_Clear` (`self.PointNearbyPlayer`))
  (for _array_element (`self.All Point Destinations`)
    (bind _output_get (set `self.ActuallyNearbyPoint` _array_element))
    (bind _returnvalue (`self.GetTransform` (stale `self.ReceiveBeginPlay` _returnvalue)))
    (bind (_returnvalue_x_2 _returnvalue_y_2 _returnvalue_z_2) (`KismetMathLibrary.BreakVector` (`KismetMathLibrary.TransformLocation` _returnvalue _output_get)))
    (if (< _returnvalue_z_2 (+ (- _returnvalue_z (`.SphereRadius` (`KismetSystemLibrary.GetComponentBounds` (`Character.CapsuleComponent` _playerref))) 40.0) (`self.WallHeight`)))
      (if (and (<= (`KismetArrayLibrary.Array_Length` (`self.PointNearbyPlayer`)) 2) (!= (`self.ActuallyNearbyPoint`) (`self.TempActualLocation`) :`ErrorTolerance` 10.0))
        (`KismetArrayLibrary.Array_Add` (`self.PointNearbyPlayer`) _actuallynearbypoint)
        (`KismetSystemLibrary.DrawDebugSphere` (`KismetMathLibrary.TransformLocation` _returnvalue _actuallynearbypoint) 100.0 4 (struct :`G` 1.0 :`B` 0.013964 :`A` 1.0) 90.0 10.0)))))

(fn `SortVectorsByDistance`
  (params (VectorsToSort :type "Array of Vector Structure (by ref)"))
  (locals (LastIndex :type Integer) (J :type Integer) (Swapped :type Boolean) (PlayerLocation :type "Vector Structure"))
  (bind _j (`local.J`))
  ;[1 1 1] Init des variables (pas besoin d'avoir un tableau temp, on travaille direct sur vectorsToSort)
  (set `local.LastIndex` (`KismetArrayLibrary.Array_LastIndex` VectorsToSort))
  (set `local.PlayerLocation` (`self.K2_GetActorLocation` (`GameplayStatics.GetPlayerCharacter` 0)))
  (for _index (range (`local.LastIndex`))
    (set `local.Swapped` false)
    (for _index_2 (range (+ (- (`local.LastIndex`) _index 1) 1))
      (set `local.J` _index_2)
      (if (> (`KismetMathLibrary.Vector_Distance` (`|GetArrayItem` (`local.VectorsToSort`) (`local.J`)) (`local.PlayerLocation`)) (`KismetMathLibrary.Vector_Distance` (`|GetArrayItem` (`local.VectorsToSort`) (+ (`local.J`) 1)) (`local.PlayerLocation`)))
        ;[1 1 1] On swap
        (`KismetArrayLibrary.Array_Swap` (`local.VectorsToSort`) _j (+ _j 1))
        (set `local.Swapped` true)))
    ;[1 1 1] Opti, si pas eu de swap, on arrete
    (if (not (`local.Swapped`))
      (return)))
  (return))

(fn `UserConstructionScript`)