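; BP_Fog drives a post-process material, likely a fog sphere around the player, with an adjustable radius.
; On BeginPlay it creates a dynamic instance of M_PlayerSphereInstance, applies it as a post-process blendable and sets a starting radius.
; SetRadiusToValue plays a timeline that lerps the Radius parameter to the requested value, using a resettable DoOnce to capture the starting radius.
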(event `self.ReceiveBeginPlay`
  ;[1 1 1] Get Post ProcessSettings
  (bind _returnvalue (`KismetMaterialLibrary.CreateDynamicMaterialInstance` "/Game/FX/Detection_Klemens/M_PlayerSphereInstance.M_PlayerSphereInstance"))
  (bind _output_get (set `self.PPMaterialRef` _returnvalue))
  (bind _weightedblendable (make `WeightedBlendable` 1.0 _output_get))
  (`KismetArrayLibrary.Array_Insert` (`.Array` (break `WeightedBlendables` (`.WeightedBlendables` (break `PostProcessSettings` (`PostProcessComponent.Settings` (`self.PostProcess`)))))) _weightedblendable)
  (set `PostProcessComponent.Settings` (make `PostProcessSettings` :`WeightedBlendables` (make `WeightedBlendables` (`|MakeArray` _weightedblendable))) (`self.PostProcess`))
  (`MaterialInstanceDynamic.SetScalarParameterValue` (`self.PPMaterialRef`) "Radius" 5000.0))

(event `Reset`
  ;[1 1 1] SetRadius of the post process
  (goto _label :!via `Reset`))

(event `SetRadiusToValue`
  (params (Radius :type "Float (double-precision)"))
  ;[1 1 1] SetRadius of the post process
  (`self.Reset`)
  (bind (_direction _newtrack_0) (`Timeline|Timeline`)
    (:`Update`
      (`|ExecutionSequence`
        (:`then_0`
          (`/Engine/EditorBlueprintResources/StandardMacros.DoOnce` false :!label _label
            (:`Completed`
              (bind _returnvalue (`MaterialInstanceDynamic.K2_GetScalarParameterValue` (`self.PPMaterialRef`) "Radius")))))
        (:`then_1`
          (`MaterialInstanceDynamic.SetScalarParameterValue` (`self.PPMaterialRef`) "Radius" (`KismetMathLibrary.Lerp` _returnvalue Radius _newtrack_0)))))))

(fn `UserConstructionScript`)