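; BP_Eclairs is a lightning effect Blueprint that periodically flashes a directional light.
; On BeginPlay it runs an endless delay loop that fires the Eclair event at a fixed interval.
; Eclair toggles the DirectionalLight intensity between bright and off in three short bursts with uneven gaps, using chained Delay nodes.
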(event `self.ReceiveBeginPlay`
  (`KismetSystemLibrary.Delay` 10.0 :!label _label)
  (`self.Eclair`)
  (goto _label))

(event `Eclair`
  (`LightComponent.SetIntensity` (`self.DirectionalLight`) 50.0)
  (`KismetSystemLibrary.Delay` 0.1)
  (`LightComponent.SetIntensity` (`self.DirectionalLight`) 0.0)
  (`KismetSystemLibrary.Delay` 0.7)
  (`LightComponent.SetIntensity` (`self.DirectionalLight`) 50.0)
  (`KismetSystemLibrary.Delay` 0.1)
  (`LightComponent.SetIntensity` (`self.DirectionalLight`) 0.0)
  (`KismetSystemLibrary.Delay` 0.3)
  (`LightComponent.SetIntensity` (`self.DirectionalLight`) 50.0)
  (`KismetSystemLibrary.Delay` 0.1)
  (`LightComponent.SetIntensity` (`self.DirectionalLight`) 0.0))

(fn `UserConstructionScript`)