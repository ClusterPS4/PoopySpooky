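; Game instance that persists player options and stores a checkpoint transform for respawning.
; CheckSave loads or creates the "Options" SaveGame_UI slot, then LoadOptions applies saved volumes to sound classes through SCM_Master, with the Music value driving the SFX class.
; SaveOptions writes language, AZERTY layout and volumes to that slot.
; Checkpoint records the player's location and rotation in memory only; Respawn teleports the player back there.
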(event `CheckSave`
  ;[0.6615 0.01599 0] Load Or Create
  (bind _returnvalue (`GameplayStatics.DoesSaveGameExist` "Options"))
  (if _returnvalue
    (bind _returnvalue_2 (`GameplayStatics.LoadGameFromSlot` "Options"))
    (bind _assave_game_ui (cast `/Game/Blueprints/SaveGame_UI` _returnvalue_2))
    (set `self.SaveGameRef` _assave_game_ui)
    (else
      (bind _returnvalue_3 (`GameplayStatics.CreateSaveGameObject` "/Game/Blueprints/SaveGame_UI.SaveGame_UI_C"))
      (bind _output_get (set `self.SaveGameRef` _returnvalue_3))
      (`GameplayStatics.SaveGameToSlot` _output_get "Options")))
  (`self.LoadOptions`))

(event `SaveOptions`
  (params (Language :type Boolean) (Azerty :type Boolean) (Volume :type "Float (double-precision)") (Music :type "Float (double-precision)") (Voices :type "Float (double-precision)"))
  (bind _savegameref (`self.SaveGameRef`))
  ;[0.224 0.399 1] Save & Load Option
  (set `/Game/Blueprints/SaveGame_UI.Language` Language _savegameref)
  (set `/Game/Blueprints/SaveGame_UI.Azerty` Azerty _savegameref)
  (set `/Game/Blueprints/SaveGame_UI.Volume` Volume _savegameref)
  (set `/Game/Blueprints/SaveGame_UI.Music` Music _savegameref)
  (set `/Game/Blueprints/SaveGame_UI.Voices` Voices _savegameref)
  (`GameplayStatics.SaveGameToSlot` (`self.SaveGameRef`) "Options"))

(event `LoadOptions`
  (bind (_language _azerty _volume _music _voices) (`self.GetSaveGameInfos`))
  ;[0.224 0.399 1] Save & Load Option
  (`GameplayStatics.SetSoundMixClassOverride` "/Game/SFX/SCM_Master.SCM_Master" "/Engine/EngineSounds/SFX.SFX" _music 1.0 0.2)
  (`GameplayStatics.PushSoundMixModifier` "/Game/SFX/SCM_Master.SCM_Master")
  (`GameplayStatics.SetSoundMixClassOverride` "/Game/SFX/SCM_Master.SCM_Master" "/Engine/EngineSounds/Master.Master" _volume 1.0 0.2)
  (`GameplayStatics.PushSoundMixModifier` "/Game/SFX/SCM_Master.SCM_Master")
  (`GameplayStatics.SetSoundMixClassOverride` "/Game/SFX/SCM_Master.SCM_Master" "/Engine/EngineSounds/Voice.Voice" _voices 1.0 0.2)
  (`GameplayStatics.PushSoundMixModifier` "/Game/SFX/SCM_Master.SCM_Master")
  (set `/Game/Blueprints/SaveGame_UI.Azerty` _azerty (`self.SaveGameRef`)))

(event `Checkpoint`
  (bind _playerref (`self.PlayerRef`))
  ;[0.2604 0.06917 0.06917] Comment
  (set `self.PlayerCheckpointPoss` (`SceneComponent.K2_GetComponentLocation` (`Actor.RootComponent` _playerref)))
  (set `self.PlayerRotator` (`SceneComponent.K2_GetComponentRotation` (`Actor.RootComponent` _playerref))))

(event `Respawn`
  ;[0.2604 0.06917 0.06917] Comment
  (`SceneComponent.K2_SetWorldLocationAndRotation` (`Actor.RootComponent` (`self.PlayerRef`)) (`self.PlayerCheckpointPoss`) (`self.PlayerRotator`) false true))

(fn `GetSaveGameInfos`
  (returns (Language :type Boolean) (Azerty :type Boolean) (Volume :type "Float (double-precision)") (Music :type "Float (double-precision)") (Voices :type "Float (double-precision)"))
  (bind _savegameref (`self.SaveGameRef`))
  (return (`/Game/Blueprints/SaveGame_UI.Language` _savegameref) (`/Game/Blueprints/SaveGame_UI.Azerty` _savegameref) (`/Game/Blueprints/SaveGame_UI.Volume` _savegameref) (`/Game/Blueprints/SaveGame_UI.Music` _savegameref) (`/Game/Blueprints/SaveGame_UI.Voices` _savegameref)))