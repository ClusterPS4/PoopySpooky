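; Checkpoint manager actor that restores level state when the LoadMap event fires.
; LoadMap unlocks doors, spawns Bertha and Klemens, disables dialogue and room triggers, marks cinematics as played, and destroys collected keys and revealed walls via actor arrays.
; It then teleports the first-person player to a stored transform.
; If the gallery is done it reveals paintings, and if the salon is also done it destroys the floor.
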(event `self.ReceiveBeginPlay`
  (bind _returnvalue (`GameplayStatics.GetActorOfClass` "/Game/FirstPerson/Blueprints/BP_FirstPersonCharacter.BP_FirstPersonCharacter_C"))
  (set `self.PlayerRef` _returnvalue))

(event `LoadMap`
  ;[1 1 1] UnlockDoors
  (for _array_element (`self.DoorsToUnlock`)
    (set `/Game/Blueprints/PortesEtActivateurs/BP_Door.Locked` false _array_element))
  ;[1 1 1] SpawnMonsters
  (`/Game/Bp_Trigger_Script/Spawns/BP_SpawnBertha.Spawn Bertha` (`self.SpawnBertha`))
  (`/Game/Bp_Trigger_Script/Spawns/BP_SpawnKlemens.Spawn` (`self.SpawnKlemens`))
  ;[1 1 1] Desactive triggers dialogues
  (for _array_element_2 (`self.TriggersToDesactivate`)
    (set `/Game/Bp_Trigger_Script/BP_TriggerSoundAndWidgets.Activated` false _array_element_2))
  ;[1 1 1] Désactive cinématiques
  (for _array_element_3 (`self.CineHasPlayed`)
    (set `/Game/Bp_Trigger_Script/BP_CameraTrigger.HasPlayed` true _array_element_3))
  ;[1 1 1] Désactive trigger de spawn
  (for _array_element_4 (`self.PaintRoomToDesactivate`)
    (set `/Game/Bp_Trigger_Script/TriggerPaintRoom.Activated` false _array_element_4))
  ;[1 1 1] Détruit clefs ramassées
  (for _array_element_5 (`self.KeysToDestroy`)
    (`self.K2_DestroyActor` _array_element_5))
  ;[1 1 1] Détruit les murs révélés
  (for _array_element_6 (`self.WallToBreak`)
    (`self.K2_DestroyActor` _array_element_6))
  ;[1 1 1] PlayerTP
  (`SceneComponent.K2_SetWorldLocationAndRotation` (`Character.CapsuleComponent` (`self.PlayerRef`)) (`self.PlayerLoc`) (`self.PlayerRot`) false false)
  ;[1 1 1] RevealDesTableaux si gallerie finie
  (if (`self.GalleryDone`)
    (for _array_element_7 (`self.TabsToReval`)
      (`/Game/Blueprints/Miroirs/BP_Tableau.Reveal` _array_element_7))
    ;[1 1 1] DestroyFloor
    (if (`self.SalonDone`)
      (`self.K2_DestroyActor` (`self.FLoorBroke`)))))

(fn `UserConstructionScript`)