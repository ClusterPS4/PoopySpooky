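; BP_LivreIndice is an interactable clue book, filed under the gallery puzzle, that shows the WG_Indice widget on screen.
; Interactable creates the widget once, then, if Activable, moves input from the interacting actor to the book and displays the widget.
; While the book has input, IA_Interract removes the widget and returns input to the stored actor, also gated by Activable.
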(event `EnhancedInput|/Game/FirstPerson/Input/Actions/IA_Interract`
  (params (ActionValue :type Boolean) (ElapsedSeconds :type "Float (double-precision)") (TriggeredSeconds :type "Float (double-precision)") (InputAction :type "InputAction Object Reference" :default "/Game/FirstPerson/Input/Actions/IA_Interract.IA_Interract"))
  (bind _returnvalue (`GameplayStatics.GetPlayerController` 0))
  ;[1 1 1] Quitter le mode livre
  (:`Started`
    (if (`self.Activable`)
      (set `self.ModeIn` false)
      (`self.DisableInput` _returnvalue)
      (`self.EnableInput` (`self.Actor`) _returnvalue)
      (`Widget.RemoveFromParent` (`self.WidgetLivre`)))))

(event `/Game/Blueprints/BPI_Interactable.Interactable`
  (params (Actor :type "Actor Object Reference"))
  (bind _returnvalue (`GameplayStatics.GetPlayerController` 0))
  ;[1 1 1] Initialisation du widget
  (`|ExecutionSequence`
    (:`then_0`
      (if (`self.Initialize`)
        (bind _returnvalue_2 (`|CreateWidget` "/Game/Blueprints/EnigmeGallerie/WG_Indice.WG_Indice_C" (`GameplayStatics.GetPlayerController` 0)))
        (set `self.WidgetLivre` _returnvalue_2)
        (set `self.Initialize` false)))
    (:`then_1`
      ;[1 1 1] Entrer en mode livre
      (if (`self.Activable`)
        (bind _output_get (set `self.Actor` Actor))
        (`self.DisableInput` _output_get _returnvalue)
        (`self.EnableInput` _returnvalue)
        (if (not (`self.ModeIn`))
          (set `self.ModeIn` true)
          (`UserWidget.AddToViewport` (`self.WidgetLivre`) 0))))))

(fn `UserConstructionScript`)