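; Interactive puzzle mirror that the player rotates to reveal hidden objects.
; Interacting moves camera and input to the mirror, and IA_Interract hands them back to the player.
; Left and right inputs turn it 45 degrees on a timeline, box-tracing forward each update to call RevealMessage on BPI_Reveal actors.
; Construction script applies mesh and trace height; the Gilbertregardelemirroir function fires line-trace fans whose results go unused.
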(event `EnhancedInput|/Game/FirstPerson/Input/Actions/IA_Interract`
  (params (ActionValue :type Boolean) (ElapsedSeconds :type "Float (double-precision)") (TriggeredSeconds :type "Float (double-precision)") (InputAction :type "InputAction Object Reference" :default "/Game/FirstPerson/Input/Actions/IA_Interract.IA_Interract"))
  (bind _returnvalue (`GameplayStatics.GetPlayerController` 0))
  (:`Started`
    (if (`self.Activable`)
      (`PlayerController.SetViewTargetWithBlend` (`GameplayStatics.GetPlayerController` 0) (`GameplayStatics.GetPlayerCharacter` 0) 0.0 "VTBlend_Linear" 0.0 false)
      (set `self.ModeIn` false)
      (`self.DisableInput` _returnvalue)
      (`self.EnableInput` (`self.Actor`) _returnvalue))))

(event `/Game/Blueprints/BPI_Interactable.Interactable`
  (params (Actor :type "Actor Object Reference"))
  (bind _returnvalue (`GameplayStatics.GetPlayerController` 0))
  (if (`self.Activable`)
    (bind _output_get (set `self.Actor` Actor))
    (`self.DisableInput` _output_get _returnvalue)
    (`self.EnableInput` _returnvalue)
    (if (not (`self.ModeIn`))
      (`PlayerController.SetViewTargetWithBlend` (`GameplayStatics.GetPlayerController` 0) self 0.0 "VTBlend_Linear" 0.0 false)
      (set `self.ModeIn` true))))

(event `EnhancedInput|/Game/FirstPerson/Input/Actions/Miroir/IA_Right`
  (params (ActionValue :type Boolean) (ElapsedSeconds :type "Float (double-precision)") (TriggeredSeconds :type "Float (double-precision)") (InputAction :type "InputAction Object Reference" :default "/Game/FirstPerson/Input/Actions/Miroir/IA_Right.IA_Right"))
  (bind (_relativerotation_roll _relativerotation_pitch _relativerotation_yaw) (`KismetMathLibrary.BreakRotator` (`SceneComponent.RelativeRotation` (`self.Cube`))))
  (:`Started`
    (if (not (`self.Rotated`))
      (set `self.Rotated` true)
      (set `self.BaseRotate` _relativerotation_yaw)
      (set `self.RotateAngle` -45.0)
      (`self.RotateMiror`))))

(event `EnhancedInput|/Game/FirstPerson/Input/Actions/Miroir/IA_Left`
  (params (ActionValue :type Boolean) (ElapsedSeconds :type "Float (double-precision)") (TriggeredSeconds :type "Float (double-precision)") (InputAction :type "InputAction Object Reference" :default "/Game/FirstPerson/Input/Actions/Miroir/IA_Left.IA_Left"))
  (bind (_relativerotation_roll _relativerotation_pitch _relativerotation_yaw) (`KismetMathLibrary.BreakRotator` (`SceneComponent.RelativeRotation` (`self.Cube`))))
  (:`Started`
    (if (not (`self.Rotated`))
      (set `self.Rotated` true)
      (set `self.BaseRotate` _relativerotation_yaw)
      (set `self.RotateAngle` 45.0)
      (`self.RotateMiror`))))

(event `RotateMiror`
  (bind _arrow (`self.Arrow`))
  (bind _baserotate (`self.BaseRotate`))
  (bind _returnvalue (`SceneComponent.K2_GetComponentLocation` _arrow))
  (bind (_direction _newtrack_0) (`Timeline|Rotate` :!via `PlayFromStart`)
    (:`Update`
      (`|ExecutionSequence`
        (:`then_0`
          (`SceneComponent.K2_SetRelativeRotation` (`self.Cube`) (`KismetMathLibrary.MakeRotator` 0.0 0.0 (`KismetMathLibrary.Lerp` _baserotate (+ _baserotate (`self.RotateAngle`)) _newtrack_0)) false false))
        (:`then_1`
          ;[1 1 1] Raycast pour reveler les objets
          (bind _outhit (`KismetSystemLibrary.BoxTraceSingle` :`Start` _returnvalue :`End` (+ _returnvalue (* (`KismetMathLibrary.GetForwardVector` (`SceneComponent.K2_GetComponentRotation` _arrow)) (`self.RayCastDist`))) :`HalfSize` (50.0 50.0 50.0) :`TraceChannel` "TraceTypeQuery1" :`DrawDebugType` "ForOneFrame"))
          (if (and (`GameplayStatics.BreakHitResult` _outhit) (`KismetSystemLibrary.DoesImplementInterface` (`.HitActor` (`GameplayStatics.BreakHitResult` _outhit)) "/Game/Blueprints/BPI_Reveal.BPI_Reveal_C"))
            (message `/Game/Blueprints/BPI_Reveal.Reveal` (`.HitActor` (`GameplayStatics.BreakHitResult` _outhit)))))
        (:`then_2`
          (set `self.Rotated` false))))))

(fn `gilbertregardelemirroir`
  (bind _returnvalue (`SceneComponent.K2_GetComponentLocation` (`self.Cube`)))
  (bind _returnvalue_2 (`SceneComponent.K2_GetComponentLocation` (`self.Cube`)))
  (bind (_returnvalue_x _returnvalue_y _returnvalue_z) (`KismetMathLibrary.BreakVector` (`KismetMathLibrary.Vector_ToDegrees` (`SceneComponent.GetForwardVector` (`self.Cube`)))))
  (bind (_returnvalue_x_2 _returnvalue_y_2 _returnvalue_z_2) (`KismetMathLibrary.BreakVector` (`KismetMathLibrary.Vector_ToDegrees` (* (`SceneComponent.GetForwardVector` (`self.Cube`)) -1.0))))
  (for _index (range 1 33)
    (`KismetSystemLibrary.LineTraceSingle` _returnvalue (+ _returnvalue (* (`KismetMathLibrary.MakeVector` (+ (* _index 4) _returnvalue_x) _returnvalue_y _returnvalue_z) 2500.0)) "TraceTypeQuery1"))
  (for _index_2 (range 1 33)
    (`KismetSystemLibrary.LineTraceSingle` _returnvalue_2 (+ _returnvalue_2 (* (`KismetMathLibrary.MakeVector` (+ (* _index_2 4) _returnvalue_x_2) _returnvalue_y_2 _returnvalue_z_2) 5000.0)) "TraceTypeQuery1")))

(fn `UserConstructionScript`
  (bind _miroirasset (`self.MiroirAsset`))
  (`SceneComponent.K2_SetRelativeLocation` (`self.Arrow`) (`KismetMathLibrary.MakeVector` 0.0 0.0 (`self.RayCastOriginHeight`)) false false)
  (`SceneComponent.SetVisibility` (`self.Cube`) false false)
  (`StaticMeshComponent.SetStaticMesh` (`self.Miroir`) _miroirasset)
  (if (== _miroirasset "/Game/Assets/Props/S_Miror_B.S_Miror_B")
    (`SceneComponent.K2_SetRelativeTransform` (`self.Miroir`) (`KismetMathLibrary.MakeTransform` (0.0 0.0 0.0) (struct) (5.0 5.0 2.25)) false false)))