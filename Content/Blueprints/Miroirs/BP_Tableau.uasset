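; BP_Tableau is one tableau in an ordered puzzle that opens a door once four tableaux are activated.
; Its Reveal event only takes effect if the tableau is off and the player character's Tableaux array holds exactly TabIndex minus one entries, enforcing the sequence.
; Activation swaps the cube's material and adds TabNum to that shared array, and reaching four entries unlocks and opens DoorToOpen.
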(event `/Game/Blueprints/BPI_Reveal.Reveal`
  (bind _doortoopen (`self.DoorToOpen`))
  ;[1 1 1] CheckSiLeTableauPrecedentEstActive
  (if (not (`self.IsOn`))
    (bind _asbp_first_person_character (cast `/Game/FirstPerson/Blueprints/BP_FirstPersonCharacter` (`GameplayStatics.GetPlayerCharacter` 0)))
    (if (== (`KismetArrayLibrary.Array_Length` (`/Game/FirstPerson/Blueprints/BP_FirstPersonCharacter.Tableaux` _asbp_first_person_character)) (- (`self.TabIndex`) 1))
      ;[1 1 1] AjoutDuTableauALaListe
      (set `self.IsOn` true)
      (`PrimitiveComponent.SetMaterial` (`self.Cube`) 0 "/Game/Blueprints/EnigmeCave/M_TempActive.M_TempActive")
      (bind _asbp_first_person_character_2 (cast `/Game/FirstPerson/Blueprints/BP_FirstPersonCharacter` (`GameplayStatics.GetPlayerCharacter` 0)))
      (bind _tableaux (`/Game/FirstPerson/Blueprints/BP_FirstPersonCharacter.Tableaux` _asbp_first_person_character_2))
      (`KismetArrayLibrary.Array_AddUnique` _tableaux (`self.TabNum`))
      ;[1 1 1] ActivationDuTableauEtDuBouton
      (if (== (`KismetArrayLibrary.Array_Length` _tableaux) 4)
        (set `/Game/Blueprints/PortesEtActivateurs/BP_Door.Locked` false _doortoopen)
        (`/Game/Blueprints/PortesEtActivateurs/BP_Door.OpenDoor` _doortoopen)))))

(fn `UserConstructionScript`)