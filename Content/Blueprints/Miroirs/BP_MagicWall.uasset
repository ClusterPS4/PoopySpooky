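; BP_MagicWall is a wall that erodes away while revealed and destroys itself once fully eroded.
; Reveal, gated by IsActivable, plays a timeline driving the Erosion material parameter on both wall meshes; StopReveal halts it, then reverses it after a short delay.
; The player pawn becomes owner, so Owner No See hides hint particles and glowing walls from its view.
; Construction assigns the wall mesh and hides the cube, flagging it visible in ray tracing.
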(event `self.ReceiveBeginPlay`
  (bind _asbp_first_person_character (cast `/Game/FirstPerson/Blueprints/BP_FirstPersonCharacter` (`GameplayStatics.GetPlayerPawn` 0)))
  (`self.SetOwner` _asbp_first_person_character)
  (`PrimitiveComponent.SetOwnerNoSee` (`self.NS_HintParticlesTest`) true)
  (`PrimitiveComponent.SetOwnerNoSee` (`self.GlowingWall1`) true)
  (`PrimitiveComponent.SetOwnerNoSee` (`self.GlowingWall2`) true))

(event `/Game/Blueprints/BPI_Reveal.Reveal`
  (if (`self.is activable`)
    (bind (_direction _newtrack_0) (`Timeline|Timeline` :!label _label)
      (:`Update`
        (bind _returnvalue (`KismetMathLibrary.Lerp` 0.0 1.0 _newtrack_0))
        (`MeshComponent.SetScalarParameterValueOnMaterials` (`self.Wall1`) "Erosion" _returnvalue)
        (`MeshComponent.SetScalarParameterValueOnMaterials` (`self.Wall2`) "Erosion" _returnvalue))
      (:`Finished`
        (if (>= _newtrack_0 1.0)
          (`self.K2_DestroyActor`))))))

(event `/Game/Blueprints/BPI_Reveal.StopReveal`
  (`|ExecutionSequence`
    (:`then_0`
      (goto _label :!via `Stop`))
    (:`then_1`
      (`KismetSystemLibrary.Delay` 1.0)
      (goto _label :!via `Reverse`))))

(fn `UserConstructionScript`
  (bind _cube (`self.Cube`))
  (bind _wallsprite (`self.WallSprite`))
  (`SceneComponent.SetVisibility` _cube false false)
  (`PrimitiveComponent.SetVisibleInRayTracing` _cube true)
  (`StaticMeshComponent.SetStaticMesh` (`self.Wall1`) _wallsprite)
  (`StaticMeshComponent.SetStaticMesh` (`self.Wall2`) _wallsprite))