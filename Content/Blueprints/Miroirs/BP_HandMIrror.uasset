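; BP_HandMIrror is a hand mirror pickup that highlights its mesh when play begins.
; Its PickUp event plays a sound, hides the mesh after a one-tick delay and shows a Subtitle widget with a French prompt to press A to Focus.
; After a short delay it removes the subtitle and destroys itself; no inventory or ability state is set here.
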(event `self.ReceiveBeginPlay`
  (`MeshComponent.SetScalarParameterValueOnMaterials` (`self.MirrorMesh`) "highlight" 1.0))

(event `/Game/Blueprints/Picking_Up_System/BPI_Items.PickUp`
  (`GameplayStatics.PlaySound2D` "/Game/SFX/SFX/sfx_object_mirror_get.sfx_object_mirror_get" 1.0 1.0 0.0 null null)
  (`KismetSystemLibrary.PrintString` "ItemPicked")
  (`KismetSystemLibrary.DelayUntilNextTick`)
  (`SceneComponent.SetHiddenInGame` (`self.MirrorMesh`) true false)
  (bind _returnvalue (`|CreateWidget` "/Game/LevelPrototyping/WidgetSubtitle/Subtitle.Subtitle_C"))
  (set `/Game/LevelPrototyping/WidgetSubtitle/Subtitle.Setcommand` "Appuyer sur A pour Focus" _returnvalue)
  (`UserWidget.AddToViewport` _returnvalue 0)
  (`KismetSystemLibrary.Delay` 2.0)
  (`Widget.RemoveFromParent` _returnvalue)
  (`self.K2_DestroyActor`))

(fn `UserConstructionScript`)