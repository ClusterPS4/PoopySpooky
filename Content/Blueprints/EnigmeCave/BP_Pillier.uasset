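; BP_Pillier is a cave puzzle pillar that rises into place and reveals either a key or another symbol.
; Spawn runs once while the pillar is down, using a timeline scaled by VerticalOffset to drive the root's height.
; Reveal, gated by Activated (not set here), switches the symbol to its active material, then either moves TargetKey to a fixed height or calls Appear on SymbolToReveal.
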(event `/Game/Blueprints/BPI_Reveal.Reveal`
  (bind _rootcomponent (`Actor.RootComponent` (`self.TargetKey`)))
  (bind (_returnvalue_x _returnvalue_y) (`KismetMathLibrary.BreakVector` (`SceneComponent.K2_GetComponentLocation` _rootcomponent)))
  (if (not (`self.Activated`))
    (`PrimitiveComponent.SetMaterial` (`self.Symbole`) 0 "/Game/Blueprints/EnigmeCave/M_TempActive.M_TempActive")
    (if (`self.RevealKey`)
      (`SceneComponent.K2_SetWorldLocation` _rootcomponent (`KismetMathLibrary.MakeVector` _returnvalue_x _returnvalue_y 228.0) false false)
      (else
        (`/Game/Blueprints/EnigmeCave/BP_SymboleMural.Appear` (`self.SymbolToReveal`))))))

(event `Spawn`
  (bind _defaultsceneroot (`self.DefaultSceneRoot`))
  (bind (_returnvalue_x _returnvalue_y) (`KismetMathLibrary.BreakVector` (`SceneComponent.K2_GetComponentLocation` _defaultsceneroot)))
  (if (`self.IsDown`)
    (set `self.IsDown` false)
    (bind (_direction _newtrack_0) (`Timeline|SpawnUp`)
      (:`Update`
        (`SceneComponent.K2_SetRelativeLocation` _defaultsceneroot (`KismetMathLibrary.MakeVector` _returnvalue_x _returnvalue_y (* _newtrack_0 (`self.VerticalOffset`))) false false)))))

(fn `UserConstructionScript`)