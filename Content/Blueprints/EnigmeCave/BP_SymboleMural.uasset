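; BP_SymboleMural is a wall symbol for the cave puzzle that can start hidden and triggers a linked pillar.
; The construction script hides the symbol mesh unless IsVisible is set, and Appear sets that flag and shows it.
; Reveal works only on a visible symbol, swapping its material to the active one and calling Spawn on its TargetPillar.
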(event `/Game/Blueprints/BPI_Reveal.Reveal`
  (if (`self.IsVisible`)
    (`PrimitiveComponent.SetMaterial` (`self. Symbole`) 0 "/Game/Blueprints/EnigmeCave/M_TempActive.M_TempActive")
    (`/Game/Blueprints/EnigmeCave/BP_Pillier.Spawn` (`self.TargetPillar`))))

(event `Appear`
  (if (not (`self.IsVisible`))
    (set `self.IsVisible` true)
    (`SceneComponent.SetVisibility` (`self. Symbole`) true false)))

(fn `UserConstructionScript`
  (if (not (`self.IsVisible`))
    (`SceneComponent.SetVisibility` (`self. Symbole`) false false)))