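; BP_BlockToReveal is a block hidden from the player until its Reveal event is triggered.
; On BeginPlay it makes the first-person character its owner and hides its mesh and Niagara effect through Owner No See.
; Reveal runs a timeline that only prints debug progress, then applies a solid blue material and clears Owner No See on both components.
; An IsRevealed flag, set on completion, blocks later reveals.
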(event `self.ReceiveBeginPlay`
  (bind _asbp_first_person_character (cast `/Game/FirstPerson/Blueprints/BP_FirstPersonCharacter` (`GameplayStatics.GetPlayerPawn` 0)))
  (`self.SetOwner` _asbp_first_person_character)
  (`PrimitiveComponent.SetOwnerNoSee` (`self.StaticMesh`) true)
  (`PrimitiveComponent.SetOwnerNoSee` (`self.Niagara`) true)
  (set `self.canSee` false)
  (set `self.canSeeParticles` false))

(event `/Game/Blueprints/BPI_Reveal.Reveal`
  ;[1 1 1] Reveal
  (if (not (`self.IsRevealed?`))
    (bind (_direction _newtrack_0) (`Timeline|RevealValue`)
      (:`Update`
        (`KismetSystemLibrary.PrintString` "loading")
        (`KismetSystemLibrary.PrintString` (`KismetStringLibrary.Conv_DoubleToString` _newtrack_0)))
      (:`Finished`
        (`self.SetVisibilityToPlayaer`)
        (set `self.IsRevealed?` true)))))

(fn `SetVisibilityToPlayaer`
  (if (not (`self.canSee`))
    (`PrimitiveComponent.SetMaterial` (`self.StaticMesh`) 0 "/Game/LevelPrototyping/Materials/MI_Solid_Blue.MI_Solid_Blue")
    (`PrimitiveComponent.SetOwnerNoSee` (`self.StaticMesh`) false)
    (`PrimitiveComponent.SetOwnerNoSee` (`self.Niagara`) false)
    (return)))

(fn `UserConstructionScript`)