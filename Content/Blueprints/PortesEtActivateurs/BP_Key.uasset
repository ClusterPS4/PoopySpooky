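; Key pickup that unlocks its referenced door and can start invisible until revealed, through a mirror according to the author's comments.
; When hidden, construction turns off its meshes but keeps the Key mesh visible in ray tracing; Reveal shows StaticMesh and enables interaction.
; Interacting unlocks DoorRef, hides the key and destroys it after a delay.
; Scripted keys also lock and close another door, while others show a Klemens subtitle.
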(event `/Game/Blueprints/BPI_Interactable.Interactable`
  (params (Actor :type "Actor Object Reference"))
  ;[1 1 1] Ajout Clef au player
  (if (`self.IsVisible`)
    (`|ExecutionSequence`
      (:`then_0`
        ;[1 1 1] ScriptCloseDoor
        (if (`self.IsScripted`)
          (bind _doortolock (`self.DoorToLock`)
            (:`then`
              (set `/Game/Blueprints/PortesEtActivateurs/BP_Door.Locked` true _doortolock)
              (if (`/Game/Blueprints/PortesEtActivateurs/BP_Door.Isopen` _doortolock)
                (`/Game/Blueprints/PortesEtActivateurs/BP_Door.OpenDoor` _doortolock)))
            (:`else`))))
      (:`then_1`
        (bind _doorref (`self.DoorRef`)
          (:`then`
            (set `/Game/Blueprints/PortesEtActivateurs/BP_Door.Locked` false _doorref)
            (`SceneComponent.SetHiddenInGame` (`self.  Key`) true false)
            (`|ExecutionSequence`
              (:`then_0`
                (if (not (`self.IsScripted`))
                  (`/Engine/EditorBlueprintResources/StandardMacros.DoOnce` false
                    (:`Completed`
                      (bind _returnvalue (`|CreateWidget` "/Game/LevelPrototyping/WidgetSubtitle/Subtitle.Subtitle_C"))
                      (bind _output_get (set `self.subtitile` _returnvalue))
                      (set `/Game/LevelPrototyping/WidgetSubtitle/Subtitle.TextToSet` "Klemens: \"Par ici ! Dans la chambre.\"" _output_get)
                      (`UserWidget.AddToViewport` _output_get 0)
                      (`KismetSystemLibrary.Delay` 2.0)
                      (`Widget.RemoveFromParent` _output_get)
                      (`self.K2_DestroyActor`)))))
              (:`then_1`
                (`KismetSystemLibrary.Delay` 2.0)
                (`self.K2_DestroyActor`))))
          (:`else`))))))

(event `/Game/Blueprints/BPI_Reveal.Reveal`
  ;[1 1 1] Apparition Clef Grace au Miroir
  (if (not (`self.IsVisible`))
    (`SceneComponent.SetVisibility` (`self.StaticMesh`) true false)
    (set `self.IsVisible` true)))

(fn `UserConstructionScript`
  ;[1 1 1] SetVisibility
  (if (not (`self.IsVisible`))
    (`SceneComponent.SetVisibility` (`self.  Key`) false false)
    (`PrimitiveComponent.SetVisibleInRayTracing` (`self.  Key`) true)
    (`SceneComponent.SetVisibility` (`self.StaticMesh`) false false)))