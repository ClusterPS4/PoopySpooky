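; BP_HiddenDoor is a hidden door that toggles open and closed once the player's lever code is long enough.
; Its Interactable event reads HiddenCode from the first-person character and calls OpenHiddenDoor when the length equals six, without comparing the contents.
; OpenHiddenDoor flips IsOpen and plays or reverses the Open timeline, which slides the Cube along relative X, scaled by DistMvt.
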(event `OpenHiddenDoor`
  ;[1 1 1] Open Hidden door
  (if (`self.IsOpen`)
    (set `self.IsOpen` false)
    (bind (_direction _newtrack_0) (`Timeline|Open` :!via `Reverse` :!label _label)
      (:`Update`
        (`SceneComponent.K2_SetRelativeLocation` (`self.Cube`) (`KismetMathLibrary.MakeVector` (* _newtrack_0 (`self.DistMvt`))) false false)))
    (else
      (set `self.IsOpen` true)
      (goto _label))))

(event `/Game/Blueprints/BPI_Interactable.Interactable`
  ;[1 1 1] Check si les leviers sont dans le bon mdp
  (bind _asbp_first_person_character (cast `/Game/FirstPerson/Blueprints/BP_FirstPersonCharacter` (`GameplayStatics.GetPlayerCharacter` 0)))
  (if (== (`KismetArrayLibrary.Array_Length` (`/Game/FirstPerson/Blueprints/BP_FirstPersonCharacter.HiddenCode` _asbp_first_person_character)) 6)
    (`self.OpenHiddenDoor`)))

(fn `UserConstructionScript`)