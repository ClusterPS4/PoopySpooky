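; BP_Door is an interactable door that can be locked or openable from one side only.
; Interacting toggles an unlocked door, with a Timeline scaling the yaw of the Porte component by Angle.
; One-way doors compare their Arrow's forward vector with the player's by dot product, permanently clearing OneWay when non-negative, and print that value.
; FirstUnlocked copies Locked at construction and clears on first unlocked interaction.
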(event `/Game/Blueprints/BPI_Interactable.Interactable`
  (params (Actor :type "Actor Object Reference"))
  ;[1 1 1] Verif Clef
  (if (`self.OneWay`)
    (`self.UnlockOneWay`)
    (elif (not (`self.Locked`))
      (`|ExecutionSequence`
        (:`then_0`
          (if (`self.FirstUnlocked`)
            (set `self.FirstUnlocked` false)))
        (:`then_1`
          (`self.OpenDoor`))))))

(event `OpenDoor`
  ;[1 1 1] Custom Event Open Door
  (if (`self.Isopen`)
    (set `self.Isopen` false)
    (bind (_direction _newtrack_0) (`Timeline|Timeline` :!via `Reverse` :!label _label)
      (:`Update`
        (`SceneComponent.K2_SetRelativeRotation` (`self.Porte`) (`KismetMathLibrary.MakeRotator` 0.0 0.0 (* _newtrack_0 (`self.Angle`))) false false)))
    (else
      (set `self.Isopen` true)
      (goto _label))))

(event `UnlockOneWay`
  (bind _returnvalue (`KismetMathLibrary.Dot_VectorVector` (`SceneComponent.GetForwardVector` (`self. Arrow`)) (`SceneComponent.GetForwardVector` (`Character.CapsuleComponent` (cast `/Game/FirstPerson/Blueprints/BP_FirstPersonCharacter` (`GameplayStatics.GetPlayerPawn` 0) :!pure true)))))
  ;[1 1 1] Unlock One Way Door
  (`KismetSystemLibrary.PrintString` (`KismetStringLibrary.Conv_DoubleToString` _returnvalue))
  (if (>= _returnvalue 0.0)
    (set `self.OneWay` false)
    (`self.OpenDoor`)))

(fn `UserConstructionScript`
  (set `self.FirstUnlocked` (`self.Locked`)))