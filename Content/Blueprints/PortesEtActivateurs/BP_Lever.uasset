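; Interactable lever for a hidden-code puzzle that flips between up and down, changing its rotation and material.
; The construction script sets the initial pose from LookTop.
; TargetPos tracks whether the lever is in its correct position, toggling on every interaction.
; While it is correct, its LeverNum is kept in the first-person character's HiddenCode array, registered at BeginPlay or on toggle and removed otherwise.
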(event `self.ReceiveBeginPlay`
  ;[1 1 1] Add ID du levier s'il est bon par defaut
  (if (`self.TargetPos`)
    (bind _asbp_first_person_character (cast `/Game/FirstPerson/Blueprints/BP_FirstPersonCharacter` (`GameplayStatics.GetPlayerCharacter` 0)))
    (`KismetArrayLibrary.Array_AddUnique` (`/Game/FirstPerson/Blueprints/BP_FirstPersonCharacter.HiddenCode` _asbp_first_person_character) (`self.LeverNum`))))

(event `/Game/Blueprints/BPI_Interactable.Interactable`
  (bind __levier (`self. Levier`))
  (bind __levier_2 (`self. Levier`))
  ;[1 1 1] Switch du levier entre haut et bas
  (if (`self.LookTop`)
    (set `self.LookTop` false)
    (`PrimitiveComponent.SetMaterial` __levier_2 0 "/Engine/MapTemplates/Materials/BasicAsset03.BasicAsset03")
    (`SceneComponent.K2_SetRelativeRotation` __levier_2 (struct :`Roll` -45.0) false false)
    (`self.CheckTarget`)
    (else
      (set `self.LookTop` true)
      (`PrimitiveComponent.SetMaterial` __levier 0 "/Engine/MapTemplates/Materials/BasicAsset01.BasicAsset01")
      (`SceneComponent.K2_SetRelativeRotation` __levier (struct :`Roll` 45.0) false false)
      (`self.CheckTarget`))))

(event `CheckTarget`
  ;[1 1 1] Verif et actualisation de si le levier est dans la bonne position
  (if (`self.TargetPos`)
    (set `self.TargetPos` false)
    (bind _asbp_first_person_character (cast `/Game/FirstPerson/Blueprints/BP_FirstPersonCharacter` (`GameplayStatics.GetPlayerCharacter` 0)))
    (`KismetArrayLibrary.Array_RemoveItem` (`/Game/FirstPerson/Blueprints/BP_FirstPersonCharacter.HiddenCode` _asbp_first_person_character) (`self.LeverNum`))
    (else
      (set `self.TargetPos` true)
      (bind _asbp_first_person_character_2 (cast `/Game/FirstPerson/Blueprints/BP_FirstPersonCharacter` (`GameplayStatics.GetPlayerCharacter` 0)))
      (`KismetArrayLibrary.Array_AddUnique` (`/Game/FirstPerson/Blueprints/BP_FirstPersonCharacter.HiddenCode` _asbp_first_person_character_2) (`self.LeverNum`)))))

(fn `UserConstructionScript`
  (bind __levier (`self. Levier`))
  (bind __levier_2 (`self. Levier`))
  (if (`self.LookTop`)
    (`PrimitiveComponent.SetMaterial` __levier 0 "/Engine/MapTemplates/Materials/BasicAsset01.BasicAsset01")
    (`SceneComponent.K2_SetRelativeRotation` __levier (struct :`Roll` 45.0) false false)
    (else
      (`PrimitiveComponent.SetMaterial` __levier_2 0 "/Engine/MapTemplates/Materials/BasicAsset03.BasicAsset03")
      (`SceneComponent.K2_SetRelativeRotation` __levier_2 (struct :`Roll` -45.0) false false))))