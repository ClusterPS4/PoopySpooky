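; BP_DoubleDoor is an interactable double door that can start locked and be unlocked from one side only.
; When locked, it compares its Arrow's forward vector with the player capsule's, prints the dot product, and unlocks and opens if non-negative.
; OpenDoorDouble toggles the OpenAngle timeline forward or backward, lerping the yaw of both door meshes toward Angle, with the mirrored leaf negated.
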(event `/Game/Blueprints/BPI_Interactable.Interactable`
  (params (Actor :type "Actor Object Reference"))
  (bind _returnvalue (`KismetMathLibrary.Dot_VectorVector` (`SceneComponent.GetForwardVector` (`self.Arrow`)) (`SceneComponent.GetForwardVector` (`Character.CapsuleComponent` (cast `/Game/FirstPerson/Blueprints/BP_FirstPersonCharacter` (`GameplayStatics.GetPlayerPawn` 0) :!pure true)))))
  ;[1 1 1] ChechOneWay
  (if (`self.IsLocked`)
    (`KismetSystemLibrary.PrintString` (`KismetStringLibrary.Conv_DoubleToString` _returnvalue))
    (if (>= _returnvalue 0.0)
      (set `self.IsLocked` false)
      (`self.OpenDoorDouble`))
    (else
      (`self.OpenDoorDouble`))))

(event `OpenDoorDouble`
  ;[1 1 1] Custom Event Open Door
  (if (`self.Isopen`)
    (set `self.Isopen` false)
    (bind (_direction _newtrack_0) (`Timeline|OpenAngle` :!via `Reverse` :!label _label)
      (:`Update`
        (bind _returnvalue (`KismetMathLibrary.Lerp` 0.0 (`self.Angle`) _newtrack_0))
        (`SceneComponent.K2_SetRelativeRotation` (`self.SM_Door`) (`KismetMathLibrary.MakeRotator` 0.0 0.0 _returnvalue) false false)
        (`SceneComponent.K2_SetRelativeRotation` (`self.SM_DoorMirror`) (`KismetMathLibrary.MakeRotator` 0.0 0.0 (* _returnvalue -1.0)) false false)))
    (else
      (set `self.Isopen` true)
      (goto _label))))

(fn `UserConstructionScript`)